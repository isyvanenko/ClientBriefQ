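; BP_CutsceneLAUNCH is a one-shot trigger actor that plays a cutscene when the player walks into it.
; Its Box overlap casts to BP_Ann_Player, then a DoOnce disables input, plays the CutSceneToPlay level sequence and hides the player.
; When the sequence finishes, it restores input and visibility, moves the player to the ENDLOCATION component's world position and destroys itself.
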(event OnComponentBeginOverlap(Box)
  (params (OverlappedComponent :type Primitive%20Component%20Object%20Reference) (OtherActor :type Actor%20Object%20Reference) (OtherComp :type Primitive%20Component%20Object%20Reference) (OtherBodyIndex :type Integer) (bFromSweep :type Boolean) (SweepResult :type Hit%20Result%20Structure%20%28by%20ref%29))
  (bind _asbp_ann_player (Utilities|Casting|CastToBP_Ann_Player OtherActor))
  (Variables|Default|SetAs%20BP%20Ann%20Player _asbp_ann_player)
  (Utilities|FlowControl|DoOnce false
    (:Completed
      (Input|DisableInput (Variables|Default|GetAs%20BP%20Ann%20Player) 0)
      (bind _returnvalue (Sequencer|Player|CreateLevelSequencePlayer (Variables|Default|GetCutSceneToPlay)))
      (bind _output_get (Variables|Default|SetNewVar _returnvalue))
      (bind _output_get_2 (Variables|Default|SetSequancePlayer _output_get))
      (Sequencer|Player|Play _output_get_2 :!class /Script/MovieScene.MovieSceneSequencePlayer)
      (Development|PrintString "started ")
      (Rendering|SetActorHiddenInGame _asbp_ann_player true)
      (EventDispatchers|AssignOnFinished (Variables|Default|GetSequancePlayer) (delegate Custom|OnFinished_Event)))))

(event Custom|OnFinished_Event
  (Input|EnableInput (Variables|Default|GetAs%20BP%20Ann%20Player) 0)
  (Rendering|SetActorHiddenInGame (stale OnComponentBeginOverlap(Box) _asbp_ann_player) false)
  (Transformation|SetActorLocation (stale OnComponentBeginOverlap(Box) _asbp_ann_player) (Transformation|GetWorldLocation (Variables|Default|GetEND%20LOCATION)) false false)
  (Development|PrintString "finished")
  (Actor|DestroyActor))

(event EventBeginPlay)

(event Collision|EventActorBeginOverlap
  (params (OtherActor :type Actor%20Object%20Reference)))

(event EventTick
  (params (DeltaSeconds :type Float%20%28single-precision%29)))

(fn ConstructionScript)